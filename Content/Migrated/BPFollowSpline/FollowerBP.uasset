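; Follower actor that moves a configurable static mesh along the spline of a BPSplinePath actor found in the level at BeginPlay.
; A timeline, with play rate set to the inverse of TimeToCompleteInSeconds, interpolates distance from zero to the spline's length.
; Each update sets the actor's world location and rotation from the spline at that distance.
; The construction script applies the chosen mesh to the Cube component.
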(event Custom|Move%20Object
  (bind _splinereferenced (Variables|Default|GetSplineReferenced))
  (bind _spline (Variables|/Game/Migrated/BPSplinePath.BPSplinePath_C|GetSpline _splinereferenced))
  (Components|Timeline|SetPlayRate (Variables|Default|GetMove%20Object%20T) (/ 1.0 (Variables|Default|GetTime%20To%20Complete%20%28In%20Seconds%29)))
  (bind _move_object_t (Timeline|Move%20Object%20T Play)
    (:Update
      (Transformation|SetActorTransform (Math|Transform|MakeTransform (Spline|GetLocationatDistanceAlongSpline _spline (Math|Float|Lerp 0.0 (Spline|GetSplineLength (Variables|/Game/Migrated/BPSplinePath.BPSplinePath_C|GetSpline (Variables|Default|GetSplineReferenced))) _move_object_t) "World") (Spline|GetRotationatDistanceAlongSpline _spline (Math|Float|Lerp 0.0 (Spline|GetSplineLength (Variables|/Game/Migrated/BPSplinePath.BPSplinePath_C|GetSpline (Variables|Default|GetSplineReferenced))) _move_object_t) "World") "1.000000,1.000000,1.000000")))))

(event EventBeginPlay
  (bind _returnvalue (Actor|GetActorOfClass "/Game/Migrated/BPSplinePath.BPSplinePath_C"))
  (Variables|Default|SetSplineReferenced _returnvalue)
  (CallFunction|MoveObject))

(fn ConstructionScript
  (Components|StaticMesh|SetStaticMesh (Variables|Default|GetCube) (Variables|Default|GetStaticMesh)))