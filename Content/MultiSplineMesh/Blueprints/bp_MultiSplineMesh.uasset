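; Component that builds repeated spline meshes with instanced separator meshes along a given spline on its owning actor.
; BuildSpline takes preset or custom data, optionally snaps spline points via vertical line traces, then divides the spline by section length.
; Each section gets a scaled spline mesh with tangents clamped to section length, plus a separator instance at its start.
; Wrappers set preset or location offset; custom data can be copied into the preset.
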(event EventBeginPlay)

(event EventTick
  (params (DeltaSeconds :type Float%20%28single-precision%29)))

(fn BuildSpline(FromPrefab)
  (params (SplinePreset :type Bp%20Multi%20Spline%20Mesh%20Preset%20Object%20Reference) (Spline :type Spline%20Component%20Object%20Reference))
  (Variables|Spline|SetSplinePreset SplinePreset)
  (Build|BuildSpline Spline))

(fn BuildSpline
  (params (Spline :type Spline%20Component%20Object%20Reference))
  ;[1 1 1] SetSpline
  (Variables|Default|SetSplineRef Spline)
  ;[1 1 1] Set Data from Preset
  (if (Variables|Spline|GetUseCusomData)
    (Variables|Spline|SetFinalData (Variables|Spline|GetCustomSplineData) :!label _label)
    (else
      (bind _splinepreset (Variables|Spline|GetSplinePreset)
        (:then
          (Variables|Spline|SetFinalData (Variables|/Game/MultiSplineMesh/Blueprints/bp_MultiSplineMesh_Preset.bp_MultiSplineMesh_Preset_C|GetSplineData _splinepreset)))
        (:else
          (goto _label)))))
  (Utilities|FlowControl|Sequence
    (:then_0
      ;[1 1 1] AutoSnap
      (if (Variables|Snapping|GetAutoSnap)
        (Editor|Snap)))
    (:then_1
      ;[1 1 1] Add Seperator
      (bind _returnvalue (Game|AddComponentbyClass (Components|GetOwner) "/Script/Engine.InstancedStaticMeshComponent" false))
      (bind _output_get (Variables|Default|SetSeperatorComp _returnvalue))
      (Components|StaticMesh|SetStaticMesh _output_get (.SeperatorMesh (Utilities|Struct|Breakst_MultiSplineMeshData (Variables|Spline|GetFinalData))))
      ;[1 1 1] BuildSpline
      ;;[0 1 0.5204] For Each Point
      (for _index (range 0 (- (Math|Float|Round (/ (Spline|GetSplineLength (Variables|Default|GetSplineRef)) (.SectionLength (Utilities|Struct|Breakst_MultiSplineMeshData (Variables|Spline|GetFinalData))))) 1))
        (LocalVariables|SetTempIndex _index)
        (Utilities|FlowControl|Sequence
          (:then_0
            ;;[0 0.3043 1] Add Spline Mesh
            (Utilities|IsValid (.sectionmesh (Variables|Spline|GetFinalData)) ; Don't build if invalid Section mesh
              (:Is%20Valid
                (bind _returnvalue_2 (Game|AddComponentbyClass (Components|GetOwner) "/Script/Engine.SplineMeshComponent" false (Transformation|GetRelativeTransform (Variables|Default|GetSplineRef))))
                (Transformation|AttachComponentToComponent _returnvalue_2 (Transformation|GetAttachParent (Variables|Default|GetSplineRef)) "None" "SnapToTarget" "SnapToTarget" "SnapToTarget" true)
                (Components|StaticMesh|SetStaticMesh _returnvalue_2 (.SectionMesh (Utilities|Struct|Breakst_MultiSplineMeshData (Variables|Spline|GetFinalData))))
                ;;[0 0.3043 1] Set Start and End
                (SplineMesh|SetStartandEnd _returnvalue_2 (.Loc (MISC|LocalGetSplineVectors (Utilities|IndextoDistance (LocalVariables|GetTempIndex)))) (.Tan (MISC|LocalGetSplineVectors (Utilities|IndextoDistance (LocalVariables|GetTempIndex)))) (.Loc (MISC|LocalGetSplineVectors (Utilities|IndextoDistance (+ (LocalVariables|GetTempIndex) 1)))) (.Tan (MISC|LocalGetSplineVectors (Utilities|IndextoDistance (+ (LocalVariables|GetTempIndex) 1)))) true :!class /Script/Engine.SplineMeshComponent)
                ;;[0 0.3043 1] Set Scale
                (SplineMesh|SetStartScale _returnvalue_2 (.sectionscale_start (Variables|Spline|GetFinalData)) true :!class /Script/Engine.SplineMeshComponent)
                (SplineMesh|SetEndScale _returnvalue_2 (.sectionscale_end (Variables|Spline|GetFinalData)) true :!class /Script/Engine.SplineMeshComponent))))
          (:then_1
            ;;[0 0.3043 1] Add Seperator
            (Utilities|IsValid (.seperatormesh (Variables|Spline|GetFinalData)) ; Don't build if invalid Seperator mesh
              (:Is%20Valid
                (Components|InstancedStaticMesh|AddInstance (Variables|Default|GetSeperatorComp) (Math|Transform|MakeTransform (.Loc (MISC|LocalGetSplineVectors (Utilities|IndextoDistance (LocalVariables|GetTempIndex)))) (Math|Rotator|MakeRotator (.X (Math|Vector|BreakVector (* (.seperatorrotationscale (Variables|Spline|GetFinalData)) (Math|Vector|MakeVector (.Roll (Math|Rotator|BreakRotator (.Rot (MISC|LocalGetSplineVectors (Utilities|IndextoDistance (LocalVariables|GetTempIndex)))))) (.Pitch (Math|Rotator|BreakRotator (.Rot (MISC|LocalGetSplineVectors (Utilities|IndextoDistance (LocalVariables|GetTempIndex)))))) (.Yaw (Math|Rotator|BreakRotator (.Rot (MISC|LocalGetSplineVectors (Utilities|IndextoDistance (LocalVariables|GetTempIndex)))))))))) (.Y (Math|Vector|BreakVector (* (.seperatorrotationscale (Variables|Spline|GetFinalData)) (Math|Vector|MakeVector (.Roll (Math|Rotator|BreakRotator (.Rot (MISC|LocalGetSplineVectors (Utilities|IndextoDistance (LocalVariables|GetTempIndex)))))) (.Pitch (Math|Rotator|BreakRotator (.Rot (MISC|LocalGetSplineVectors (Utilities|IndextoDistance (LocalVariables|GetTempIndex)))))) (.Yaw (Math|Rotator|BreakRotator (.Rot (MISC|LocalGetSplineVectors (Utilities|IndextoDistance (LocalVariables|GetTempIndex)))))))))) (.Z (Math|Vector|BreakVector (* (.seperatorrotationscale (Variables|Spline|GetFinalData)) (Math|Vector|MakeVector (.Roll (Math|Rotator|BreakRotator (.Rot (MISC|LocalGetSplineVectors (Utilities|IndextoDistance (LocalVariables|GetTempIndex)))))) (.Pitch (Math|Rotator|BreakRotator (.Rot (MISC|LocalGetSplineVectors (Utilities|IndextoDistance (LocalVariables|GetTempIndex)))))) (.Yaw (Math|Rotator|BreakRotator (.Rot (MISC|LocalGetSplineVectors (Utilities|IndextoDistance (LocalVariables|GetTempIndex)))))))))))) false)))))))))

(fn LocalRunSnap
  (params (Start :type Vector) (End%20Z :type Float%20%28double-precision%29))
  (bind (_outhit _returnvalue) (Collision|LineTraceForObjects Start (+ Start (Math|Vector|MakeVector 0.0 0.0 End%20Z)) (Variables|Snapping|GetSnapTypes) false (Utilities|Array|MakeArray (Components|GetOwner)) "ForDuration"))
  (return _outhit _returnvalue))

(fn LocalGetSplineVectors
  (params (Distance :type Float%20%28single-precision%29))
  (bind _finaldata (Variables|Spline|GetFinalData))
  (bind _splineref (Variables|Default|GetSplineRef))
  (bind _sectionlength (Utilities|Struct|Breakst_MultiSplineMeshData _finaldata))
  (bind _returnvalue (Spline|GetRotationatDistanceAlongSpline _splineref Distance "Local"))
  (return (+ (Spline|GetLocationatDistanceAlongSpline _splineref Distance "Local") (Math|Vector|RotateVector (Variables|Spline|GetLocationOffset) _returnvalue)) (Math|Vector|ClampVectorSize (Spline|GetTangentatDistanceAlongSpline _splineref Distance "Local") _sectionlength _sectionlength) _returnvalue))

(fn Snap
  (bind _index (Utilities|ForEachSplinePoint)
    (:LoopBody
      (bind (_outhit _returnvalue) (MISC|LocalRunSnap (Spline|GetLocationatSplinePoint (Variables|Default|GetSplineRef) _index "World") (* (Variables|Snapping|GetTraceDistance) (Math|Float|SelectFloat 1.0 -1.0 (Variables|Snapping|GetTraceUp)))))
      (if _returnvalue
        (Spline|SetLocationatSplinePoint (Variables|Default|GetSplineRef) _index (.ImpactPoint (Collision|BreakHitResult _outhit)) "World" true)))))

(fn ApplyCustomDatatoPreset
  (Variables|/Game/MultiSplineMesh/Blueprints/bp_MultiSplineMesh_Preset.bp_MultiSplineMesh_Preset_C|SetSplineData (Variables|Spline|GetSplinePreset) (Variables|Spline|GetCustomSplineData)))

(fn BuildSpline(AtOffset)
  (params (Spline :type Spline%20Component%20Object%20Reference) (LocationOffset :type Vector))
  (Variables|Spline|SetLocationOffset LocationOffset)
  (Build|BuildSpline Spline))